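; Player stats component that tracks health and stamina for BP_Alien and drives the matching HUD bars.
; BeginPlay caches the owner, waits a tick, then fills both bars from current/max ratios.
; Increase and decrease functions update each bar directly, clamping values except on health damage.
; Decreases return whether the stat is depleted and healing returns whether health is full, while stamina recovery's equivalent check is disconnected.
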(event `self.ReceiveBeginPlay`
  (bind _asbp_alien (cast `/Game/Characters/My/Blueprint/BP_Alien` (`self.GetOwner`)))
  (`KismetSystemLibrary.DelayUntilNextTick`)
  (set `self.Player Character` _asbp_alien)
  (`ProgressBar.SetPercent` (`/Game/Characters/My/UI/WB_PlayerHUD.HealthBar` (`/Game/Characters/My/Blueprint/BP_Alien.HUD` (`self.Player Character`))) (/ (`self.CurrentHealth`) (`self.MaxHealth`)))
  (`ProgressBar.SetPercent` (`/Game/Characters/My/UI/WB_PlayerHUD.StaminaBar` (`/Game/Characters/My/Blueprint/BP_Alien.HUD` (`self.Player Character`))) (/ (`self.CurrentStamina`) (`self.MaxStamina`))))

(event `self.ReceiveTick`
  (params (DeltaSeconds :type "Float (single-precision)")))

(fn `DecreasePlayerHealth`
  (params (DamageAmount :type "Float (double-precision)"))
  (returns (`IsPlayerDead?` :type Boolean))
  (bind _currenthealth (`self.CurrentHealth`))
  (if (> _currenthealth 0.0)
    (bind _output_get (set `self.CurrentHealth` (- _currenthealth DamageAmount)))
    (`ProgressBar.SetPercent` (`/Game/Characters/My/UI/WB_PlayerHUD.HealthBar` (`/Game/Characters/My/Blueprint/BP_Alien.HUD` (`self.Player Character`))) (/ _output_get (`self.MaxHealth`)))
    (if (<= (`self.CurrentHealth`) 0.0)
      (return true)
      (else
        (return false)))
    (else
      (return true))))

(fn `DecreasePlayerStamina`
  (params (StaminaConsumption :type "Float (double-precision)"))
  (returns (`NoStamina?` :type Boolean))
  (bind _currentstamina (`self.CurrentStamina`))
  (if (not (<= _currentstamina 0.0))
    (bind _output_get (set `self.CurrentStamina` (`KismetMathLibrary.FClamp` (- _currentstamina StaminaConsumption) 0.0 (`self.MaxStamina`))))
    (`ProgressBar.SetPercent` (`/Game/Characters/My/UI/WB_PlayerHUD.StaminaBar` (`/Game/Characters/My/Blueprint/BP_Alien.HUD` (`self.Player Character`))) (/ _output_get (`self.MaxStamina`)))
    (if (<= (`self.CurrentStamina`) 0.0)
      _
      (else
        (return false))))
  (return true))

(fn `GetCurrentHealth`
  (returns (Health :type "Float (double-precision)"))
  (return (`self.CurrentHealth`)))

(fn `IncreasePlayerHealth`
  (params (HealingAmount :type "Float (double-precision)"))
  (returns (IsHealthFull :type Boolean))
  (bind _maxhealth (`self.MaxHealth`))
  (bind _output_get (set `self.CurrentHealth` (`KismetMathLibrary.FClamp` (+ (`self.CurrentHealth`) HealingAmount) 0.0 (`self.MaxHealth`))))
  (`ProgressBar.SetPercent` (`/Game/Characters/My/UI/WB_PlayerHUD.HealthBar` (`/Game/Characters/My/Blueprint/BP_Alien.HUD` (`self.Player Character`))) (/ _output_get _maxhealth))
  (if (== _output_get _maxhealth)
    (return true)
    (else
      (return false))))

(fn `IncreasePlayerStamina`
  (params (StaminaRecovery :type "Float (double-precision)"))
  (returns (`IsStaminaFull?` :type Boolean))
  (if (< (`self.CurrentStamina`) (`self.MaxStamina`))
    (bind _output_get (set `self.CurrentStamina` (`KismetMathLibrary.FClamp` (+ StaminaRecovery (`self.CurrentStamina`)) 0.0 (`self.MaxStamina`))))
    (`ProgressBar.SetPercent` (`/Game/Characters/My/UI/WB_PlayerHUD.StaminaBar` (`/Game/Characters/My/Blueprint/BP_Alien.HUD` (`self.Player Character`))) (/ _output_get (`self.MaxStamina`)))))