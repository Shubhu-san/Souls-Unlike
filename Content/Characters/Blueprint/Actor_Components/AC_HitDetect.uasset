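; AC_HitDetect is an actor component on BP_Alien that detects sword hits on enemies and applies damage.
; TraceHit sphere-traces between the owner's SwordTop and SwordBottom and reacts only to actors tagged Enemy.
; A hit deals fixed damage and spawns a spark emitter at the impact, deactivated shortly after.
; A DoOnce gate, reset after short delays, prevents repeated hits during a swing.
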(event `self.ReceiveBeginPlay`
  (bind _asbp_alien (cast `/Game/Characters/Blueprint/BP_Alien` (`self.GetOwner`)))
  (`KismetSystemLibrary.DelayUntilNextTick`)
  (set `self.Player Character` _asbp_alien))

(event `TraceHit`
  (bind _player_character (`self.Player Character`))
  (bind (_outhit _returnvalue) (`KismetSystemLibrary.SphereTraceSingle` :`Start` (`SceneComponent.K2_GetComponentLocation` (`/Game/Characters/Blueprint/BP_Alien.SwordTop` _player_character)) :`End` (`SceneComponent.K2_GetComponentLocation` (`/Game/Characters/Blueprint/BP_Alien.SwordBottom` _player_character)) :`Radius` 6.5 :`TraceChannel` "TraceTypeQuery1" :`DrawTime` 0.5))
  (if _returnvalue
    (bind (_bblockinghit _binitialoverlap _time _distance _location _impactpoint _normal _impactnormal _physmat _hitactor) (`GameplayStatics.BreakHitResult` _outhit))
    (if (`Actor.ActorHasTag` _hitactor "Enemy")
      (`/Engine/EditorBlueprintResources/StandardMacros.DoOnce` false :!label _label
        (:`Completed`
          (`GameplayStatics.ApplyDamage` _hitactor 30.0)
          (bind _returnvalue_2 (`GameplayStatics.SpawnEmitterAtLocation` "/Game/VFX/Particles/Sparks/P_Sparks_C.P_Sparks_C" _location (`KismetMathLibrary.MakeRotFromXY` _normal _normal) (0.5 0.5 0.5) true "AutoRelease"))
          (bind _output_get (set `self.SparkEmitter` _returnvalue_2))
          (`KismetSystemLibrary.Delay` 0.5)
          (`self.Deactivate` _output_get)
          (`KismetSystemLibrary.Delay` 0.5)
          (goto _label :!via `Reset`))))))