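; Actor component that tracks health and stamina and, despite its name, serves the player alien, normie NPCs and bosses.
; On BeginPlay it casts the owner to identify its type, waits a tick, then initializes the matching UI bars.
; Damage updates the owner's health bar and reports depletion.
; Healing and stamina changes write directly to the player HUD, so they assume a player owner.
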(event `self.ReceiveBeginPlay`
  (bind _returnvalue (`self.GetOwner`))
  (bind _asbp_alien (cast `/Game/Characters/Blueprint/BP_Alien` _returnvalue)
    (:`then`
      (`KismetSystemLibrary.DelayUntilNextTick`)
      (set `self.IsPlayer` true)
      (set `self.Player Character` _asbp_alien)
      (`ProgressBar.SetPercent` (`/Game/UI/PlayerUI/WB_PlayerHUD.StaminaBar` (`/Game/Characters/Blueprint/BP_Alien.HUD` (`self.Player Character`))) (/ (`self.CurrentStamina`) (`self.MaxStamina`))))
    (:`CastFailed`
      (bind _asbp_normie_npc (cast `/Game/AI/Normie/BP_NormieNPC` _returnvalue)
        (:`then`
          (`KismetSystemLibrary.DelayUntilNextTick`)
          (set `self.IsPlayer` false)
          (set `self.IsBoss` false)
          (bind _output_get (set `self.As BP Normie` _asbp_normie_npc)))
        (:`CastFailed`
          (bind _asbp_boss_npc (cast `/Game/AI/Boss/BP_BossNPC` _returnvalue))
          (`KismetSystemLibrary.DelayUntilNextTick`)
          (set `self.IsBoss` true)
          (bind _output_get_2 (set `self.As BP Boss NPC` _asbp_boss_npc))))))
  (`ProgressBar.SetPercent` (select `bool` (`self.IsBoss`) :`false` (select `bool` (`self.IsPlayer`) :`false` (`/Game/UI/EnemyUI/WB_EnemyUI.HP_Bar` (`/Game/AI/Normie/BP_NormieNPC.EnemyUI` _output_get)) :`true` (`/Game/UI/PlayerUI/WB_PlayerHUD.HealthBar` (`/Game/Characters/Blueprint/BP_Alien.HUD` (`self.Player Character`)))) :`true` (`/Game/UI/BossUI/Boss_HUD.HP_Bar` (`/Game/AI/Boss/BP_BossNPC.BossHUD` _output_get_2))) (/ (`self.CurrentHealth`) (`self.MaxHealth`))))

(event `self.ReceiveTick`
  (params (DeltaSeconds :type "Float (single-precision)")))

(fn `DecreasePlayerHealth`
  (params (DamageAmount :type "Float (double-precision)"))
  (returns (`IsPlayerDead?` :type Boolean))
  (bind _currenthealth (`self.CurrentHealth`))
  (if (> _currenthealth 0.0)
    (bind _output_get (set `self.CurrentHealth` (- _currenthealth DamageAmount)))
    (`ProgressBar.SetPercent` (select `bool` (`self.IsBoss`) :`false` (select `bool` (`self.IsPlayer`) :`false` (`/Game/UI/EnemyUI/WB_EnemyUI.HP_Bar` (`/Game/AI/Normie/BP_NormieNPC.EnemyUI` (`self.As BP Normie`))) :`true` (`/Game/UI/PlayerUI/WB_PlayerHUD.HealthBar` (`/Game/Characters/Blueprint/BP_Alien.HUD` (`self.Player Character`)))) :`true` (`/Game/UI/BossUI/Boss_HUD.HP_Bar` (`/Game/AI/Boss/BP_BossNPC.BossHUD` (`self.As BP Boss NPC`)))) (/ _output_get (`self.MaxHealth`)))
    (if (<= (`self.CurrentHealth`) 0.0)
      (return true)
      (else
        (return false)))
    (else
      (return true))))

(fn `DecreasePlayerStamina`
  (params (StaminaConsumption :type "Float (double-precision)"))
  (returns (`NoStamina?` :type Boolean))
  (bind _currentstamina (`self.CurrentStamina`))
  (if (not (<= _currentstamina 0.0))
    (bind _output_get (set `self.CurrentStamina` (`KismetMathLibrary.FClamp` (- _currentstamina StaminaConsumption) 0.0 (`self.MaxStamina`))))
    (`ProgressBar.SetPercent` (`/Game/UI/PlayerUI/WB_PlayerHUD.StaminaBar` (`/Game/Characters/Blueprint/BP_Alien.HUD` (`self.Player Character`))) (/ _output_get (`self.MaxStamina`)))
    (if (<= (`self.CurrentStamina`) 0.0)
      _
      (else
        (return false))))
  (return true))

(fn `GetCurrentHealth`
  (returns (Health :type "Float (double-precision)"))
  (return (`self.CurrentHealth`)))

(fn `GetCurrentStamina`
  (returns (Health :type "Float (double-precision)"))
  (return (`self.CurrentStamina`)))

(fn `IncreasePlayerHealth`
  (params (HealingAmount :type "Float (double-precision)"))
  (returns (IsHealthFull :type Boolean))
  (bind _maxhealth (`self.MaxHealth`))
  (bind _output_get (set `self.CurrentHealth` (`KismetMathLibrary.FClamp` (+ (`self.CurrentHealth`) HealingAmount) 0.0 (`self.MaxHealth`))))
  (`ProgressBar.SetPercent` (`/Game/UI/PlayerUI/WB_PlayerHUD.HealthBar` (`/Game/Characters/Blueprint/BP_Alien.HUD` (`self.Player Character`))) (/ _output_get _maxhealth))
  (if (== _output_get _maxhealth)
    (return true)
    (else
      (return false))))

(fn `IncreasePlayerStamina`
  (params (StaminaRecovery :type "Float (double-precision)"))
  (returns (`IsStaminaFull?` :type Boolean))
  (if (< (`self.CurrentStamina`) (`self.MaxStamina`))
    (bind _output_get (set `self.CurrentStamina` (`KismetMathLibrary.FClamp` (+ StaminaRecovery (`self.CurrentStamina`)) 0.0 (`self.MaxStamina`))))
    (`ProgressBar.SetPercent` (`/Game/UI/PlayerUI/WB_PlayerHUD.StaminaBar` (`/Game/Characters/Blueprint/BP_Alien.HUD` (`self.Player Character`))) (/ _output_get (`self.MaxStamina`)))))