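; BP_Dummy is a damageable enemy character that reacts to hits with montages and knockback along the player's facing direction.
; Damage feeds its ACPlayerStats component through DecreasePlayerHealth, whose true result triggers death: hidden UI, death montage, stronger launch, kill sound and delayed destruction.
; BeginPlay caches the WB_EnemyUI widget from HpBar, which turns toward the camera every Tick.
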(event `self.ReceiveAnyDamage`
  (params (Damage :type "Float (single-precision)") (DamageType :type "DamageType Object Reference") (InstigatedBy :type "Controller Object Reference") (DamageCauser :type "Actor Object Reference"))
  (bind _returnvalue (`GameplayStatics.GetPlayerCharacter` 0))
  (`self.PlayAnimMontage` "/Game/Characters/Animation/Actions/AM_Hit_ImpactEnemy.AM_Hit_ImpactEnemy")
  (cast `/Game/Characters/Blueprint/BP_Alien` _returnvalue)
  (`self.LaunchCharacter` (* (`KismetMathLibrary.GetForwardVector` (`self.K2_GetActorRotation` _returnvalue)) 250.0))
  (bind _isplayerdead_ (`/Game/Characters/Blueprint/Actor_Components/AC_PlayerStats.DecreasePlayerHealth` (`self.AC_PlayerStats`) Damage))
  (if _isplayerdead_
    (set `Widget.Visibility` "Hidden" (`self.EnemyUI`))
    (`self.PlayAnimMontage` "/Game/Characters/Animation/Actions/AM_Death.AM_Death")
    (`self.LaunchCharacter` (* (`KismetMathLibrary.GetForwardVector` (`self.K2_GetActorRotation` (`GameplayStatics.GetPlayerCharacter` 0))) 700.0))
    (`GameplayStatics.PlaySoundAtLocation` "/Game/Characters/Audio/Hit_Death/MS_Killed.MS_Killed" (`self.K2_GetActorLocation`) (struct) 1.0 1.0 0.0 null null null null)
    (`KismetSystemLibrary.Delay` 2.0)
    (`self.K2_DestroyActor`)))

(event `self.ReceiveTick`
  (params (DeltaSeconds :type "Float (single-precision)"))
  (bind _hp_bar (`self.Hp_Bar`))
  (`SceneComponent.K2_SetWorldRotation` _hp_bar (`KismetMathLibrary.FindLookAtRotation` (`SceneComponent.K2_GetComponentLocation` _hp_bar) (`SceneComponent.K2_GetComponentLocation` (`PlayerCameraManager.TransformComponent` (`GameplayStatics.GetPlayerCameraManager` 0)))) false false))

(event `self.ReceiveBeginPlay`
  (bind _aswb_enemy_ui (cast `/Game/UI/EnemyUI/WB_EnemyUI` (`WidgetComponent.GetWidget` (`self.Hp_Bar`))))
  (set `self.EnemyUI` _aswb_enemy_ui))

(fn `UserConstructionScript`)