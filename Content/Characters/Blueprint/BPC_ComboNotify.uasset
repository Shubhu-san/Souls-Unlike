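; Anim notify state that marks a combo window in an animation for the player's alien character.
; On begin it passes its LightAttack and HeavyAttack values to BP_Alien's AttackType, and on end it calls DefaultAttack.
; It targets player 0's character rather than the animated mesh's owner, and does nothing if that character is not a BP_Alien.
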(fn `Received_NotifyBegin`
  (params (MeshComp :type "SkeletalMeshComponent Object Reference") (Animation :type "AnimSequenceBase Object Reference") (TotalDuration :type "Float (single-precision)") (EventReference :type "AnimNotifyEventReference Structure (by ref)"))
  (returns (ReturnValue :type Boolean))
  (bind _asbp_alien (cast `/Game/Characters/Blueprint/BP_Alien` (`GameplayStatics.GetPlayerCharacter` MeshComp)))
  (`/Game/Characters/Blueprint/BP_Alien.AttackType` _asbp_alien (`self.Light Attack`) (`self.Heavy Attack`))
  (return true))

(fn `Received_NotifyEnd`
  (params (MeshComp :type "SkeletalMeshComponent Object Reference") (Animation :type "AnimSequenceBase Object Reference") (EventReference :type "AnimNotifyEventReference Structure (by ref)"))
  (returns (ReturnValue :type Boolean))
  (bind _asbp_alien (cast `/Game/Characters/Blueprint/BP_Alien` (`GameplayStatics.GetPlayerCharacter` MeshComp)))
  (`/Game/Characters/Blueprint/BP_Alien.DefaultAttack` _asbp_alien)
  (return true))

(fn `Received_NotifyTick`
  (params (MeshComp :type "SkeletalMeshComponent Object Reference") (Animation :type "AnimSequenceBase Object Reference") (FrameDeltaTime :type "Float (single-precision)") (EventReference :type "AnimNotifyEventReference Structure (by ref)"))
  (returns (ReturnValue :type Boolean)))