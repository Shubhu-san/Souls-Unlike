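; BPC_DamageSystem is a damage component that tracks health, healing, blocking and death for its owner.
; TakeDamage uses the CanBeDamaged macro to choose block, damage or ignore from dead, invincible and blocking states plus the hit's override flags.
; It calls OnBlocked, OnDeath, or OnDamageResponse when a non-lethal hit can interrupt, leaving reactions to listeners.
; Heal adds health clamped to MaxHealth unless dead.
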(fn `Heal`
  (params (HealingAmount :type "Float (double-precision)"))
  (returns (`New Health` :type "Float (double-precision)"))
  (if (`self.IsDead`)
    _
    (elif (== (`self.Health`) (`self.MaxHealth`))
      (return (`self.Health`))
      (else
        (bind _output_get (set `self.Health` (`KismetMathLibrary.FClamp` (+ HealingAmount (`self.Health`)) 0.0 (`self.MaxHealth`))))
        (return _output_get)))))

(fn `TakeDamage`
  (params (NewParam :type "/Game/DamageSystem/S_DamageInfo Structure"))
  (returns (isDamaged :type Boolean))
  (bind (_damageamount _damagetype _damageresponse _shoulddamageinvincible _canbeblocked _canbeparried _shouldforceinterrupt) (break `/Game/DamageSystem/S_DamageInfo` NewParam))
  (`self.CanBeDamaged` _shoulddamageinvincible _canbeblocked
    (:`BlockDamage`
      (`self.OnBlocked` _canbeparried)
      (return false))
    (:`DoDamage`
      (bind _output_get (set `self.Health` (- (`self.Health`) _damageamount)))
      (if (<= _output_get 0.0)
        (set `self.IsDead` true)
        (`self.OnDeath`)
        (return true)
        (elif (or _shouldforceinterrupt (`self.IsInterruptible`))
          (`self.OnDamageResponse` _damageresponse)
          (return true))))
    (:`NoDamage`
      (return false))))