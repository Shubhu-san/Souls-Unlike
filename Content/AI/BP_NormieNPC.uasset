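; Melee enemy NPC with a sword and a camera-facing health bar.
; Attack plays a random montage; an indexed three-hit combo also exists, but its CanAttack trigger is disconnected.
; TraceHit sphere-traces along the blade, applying damage and sparks to Player-tagged actors with a half-second lockout.
; Taking damage knocks it along the player's facing and drains ACPlayerStats health; death adds a stronger launch, montage and sound before destruction.
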(event `self.ReceiveAnyDamage`
  (params (Damage :type "Float (single-precision)") (DamageType :type "DamageType Object Reference") (InstigatedBy :type "Controller Object Reference") (DamageCauser :type "Actor Object Reference"))
  (bind _returnvalue (`GameplayStatics.GetPlayerCharacter` 0))
  ;[0.05098 0.05098 0.05098] Damage
  (`self.PlayAnimMontage` "/Game/Characters/Animation/Actions/AM_Hit_ImpactEnemy.AM_Hit_ImpactEnemy")
  ;;[0.05098 0.05098 0.05098] Launch Enemy on taking damage
  (cast `/Game/Characters/Blueprint/BP_Alien` _returnvalue)
  (`self.LaunchCharacter` (* (`KismetMathLibrary.GetForwardVector` (`self.K2_GetActorRotation` _returnvalue)) 250.0))
  (bind _isplayerdead_ (`/Game/Characters/Blueprint/Actor_Components/AC_PlayerStats.DecreasePlayerHealth` (`self.AC_PlayerStats`) Damage))
  (bind _output_get (set `self.Is Player Dead?` _isplayerdead_))
  (if _output_get
    ;;[0.05098 0.05098 0.05098] Enemy After Death
    (set `Widget.Visibility` "Hidden" (`self.EnemyUI`))
    (`self.PlayAnimMontage` "/Game/Characters/Animation/Actions/AM_Death.AM_Death" 1.25)
    (`self.LaunchCharacter` (* (`KismetMathLibrary.GetForwardVector` (`self.K2_GetActorRotation` (`GameplayStatics.GetPlayerCharacter` 0))) 700.0))
    (`GameplayStatics.PlaySoundAtLocation` "/Game/Characters/Audio/Hit_Death/MS_Killed.MS_Killed" (`self.K2_GetActorLocation`) (struct) 1.0 1.0 0.0 null null null null)
    (`KismetSystemLibrary.Delay` 1.0)
    (`self.K2_DestroyActor`)))

(event `self.ReceiveTick`
  (params (DeltaSeconds :type "Float (single-precision)"))
  (bind _hp_bar (`self.Hp_Bar`))
  ;[0.05098 0.05098 0.05098] Health Bar Face Camera
  (`SceneComponent.K2_SetWorldRotation` _hp_bar (`KismetMathLibrary.FindLookAtRotation` (`SceneComponent.K2_GetComponentLocation` _hp_bar) (`SceneComponent.K2_GetComponentLocation` (`PlayerCameraManager.TransformComponent` (`GameplayStatics.GetPlayerCameraManager` 0)))) false false))

(event `self.ReceiveBeginPlay`
  ;[0.05098 0.05098 0.05098] Get Health Bar UI
  (bind _aswb_enemy_ui (cast `/Game/Characters/UI/EnemyUI/WB_EnemyUI` (`WidgetComponent.GetWidget` (`self.Hp_Bar`))))
  (set `self.EnemyUI` _aswb_enemy_ui))

(event `Attack 1`
  ;[0.05098 0.05098 0.05098] Attack On Melee Range
  (`/Engine/EditorBlueprintResources/StandardMacros.DoOnce` false :!label _label
    (:`Completed`
      (`KismetSystemLibrary.Delay` 0.1)
      (`|PlayMontage` (`self.Mesh`) "/Game/Characters/Animation/Attacks/Light/Ai/Attack1.Attack1"
        (:`then`
          (set `self.AttackIndex` 1)
          (goto _label :!via `Reset`))))))

(event `Ai Attack`
  ;[1 1 1] Can Attack
)

(event `Attack 2`
  ;[0.05098 0.05098 0.05098] Attack On Melee Range
  (`/Engine/EditorBlueprintResources/StandardMacros.DoOnce` false :!label _label_2
    (:`Completed`
      (`KismetSystemLibrary.Delay` 0.1)
      (`|PlayMontage` (`self.Mesh`) "/Game/Characters/Animation/Attacks/Light/Ai/Attack2.Attack2"
        (:`then`
          (set `self.AttackIndex` 2)
          (goto _label_2 :!via `Reset`))))))

(event `Sword Attack`
  ;[1 1 1] Sword Attack
  (if (`self.Is Attacking`)
    (set `self.saveAttack?` true)
    (else
      (set `self.Is Attacking` true)
      (switch `int` (`self.AttackIndex`) :!label _label_3
        (:`0`
          (`self.Attack 1`))
        (:`1`
          (`self.Attack 2`))
        (:`2`
          (`self.Attack 3`))))))

(event `Attack 3`
  ;[0.05098 0.05098 0.05098] Attack On Melee Range
  (`/Engine/EditorBlueprintResources/StandardMacros.DoOnce` false :!label _label_4
    (:`Completed`
      (`KismetSystemLibrary.Delay` 0.1)
      (`|PlayMontage` (`self.Mesh`) "/Game/Characters/Animation/Attacks/Light/Ai/Attack3.Attack3"
        (:`then`
          (set `self.AttackIndex` 0)
          (goto _label_4 :!via `Reset`))))))

(event `Sword Attack Combo`
  ;[1 1 1] Continue Combo
  (if (`self.saveAttack?`)
    (set `self.saveAttack?` false)
    (goto _label_3)))

(event `Stop Combo`
  ;[1 1 1] Stop Combo
  (set `self.Is Attacking` false)
  (set `self.AttackIndex` 0))

(event `TraceHit`
  ;[1 1 1] Sword Trace
  (bind (_outhit _returnvalue) (`KismetSystemLibrary.SphereTraceSingle` :`Start` (`SceneComponent.K2_GetComponentLocation` (`self.SwordTop`)) :`End` (`SceneComponent.K2_GetComponentLocation` (`self.SwordBottom`)) :`Radius` 6.5 :`TraceChannel` "TraceTypeQuery1" :`DrawTime` 1.0))
  (if _returnvalue
    (bind (_bblockinghit _binitialoverlap _time _distance _location _impactpoint _normal _impactnormal _physmat _hitactor) (`GameplayStatics.BreakHitResult` _outhit))
    (if (`self.ActorHasTag` _hitactor "Player")
      (`/Engine/EditorBlueprintResources/StandardMacros.DoOnce` false :!label _label_5
        (:`Completed`
          (`GameplayStatics.ApplyDamage` _hitactor (`self.Base Damage`))
          (bind _returnvalue_2 (`GameplayStatics.SpawnEmitterAtLocation` "/Game/VFX/Particles/Sparks/P_Sparks_C.P_Sparks_C" _location (`KismetMathLibrary.MakeRotFromXY` _normal _normal) (0.5 0.5 0.5) true "AutoRelease"))
          (bind _output_get (set `self.SparkEmitter` _returnvalue_2))
          (`KismetSystemLibrary.Delay` 0.5)
          (`ActorComponent.Deactivate` _output_get)
          (goto _label_5 :!via `Reset`))))))

(event `Attacks`
  (bind _attackanims (`self.AttackAnims`))
  ;[1 1 1] AI COMBO ATTACKS
  (`/Engine/EditorBlueprintResources/StandardMacros.DoOnce` false :!label _label_6
    (:`Completed`
      (`|PlayMontage` (`self.Mesh`) (`|GetArrayItem` _attackanims (`KismetMathLibrary.RandomInteger` (`KismetArrayLibrary.Array_Length` _attackanims)))
        (:`OnCompleted`
          (goto _label_6 :!via `Reset`))
        (:`OnInterrupted`
          (`KismetSystemLibrary.Delay` 1.0)
          (goto _label_6 :!via `Reset`))))))

(fn `Attack`
  (returns (`Anim Duration` :type "Float (double-precision)"))
  (`self.Attacks`)
  (return 0.4))

(fn `UserConstructionScript`)