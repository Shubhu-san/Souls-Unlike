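; Boss enemy character that fights the player with random mace attack montages and shows a HUD created on BeginPlay.
; Attack triggers a gated, randomly delayed montage, while TraceHit sphere-traces along the mace to damage the player and spawn sparks.
; Damage knocks the boss back and feeds ACPlayerStats, whose death result (stored as IsPlayerDead despite meaning the boss) triggers BossDeath and destruction.
; Tick keeps the whole actor facing the player.
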(event `self.ReceiveAnyDamage`
  (params (Damage :type "Float (single-precision)") (DamageType :type "DamageType Object Reference") (InstigatedBy :type "Controller Object Reference") (DamageCauser :type "Actor Object Reference"))
  (bind _returnvalue (`GameplayStatics.GetPlayerCharacter` 0))
  (bind _damagetaken (`/Game/UI/BossUI/Boss_HUD.DamageTaken` (`self.BossHUD`)))
  ;[0.05098 0.05098 0.05098] Damage
  (`self.PlayAnimMontage` "/Game/Characters/Animation/Actions/AM_Hit_ImpactEnemy.AM_Hit_ImpactEnemy")
  ;;[0.05098 0.05098 0.05098] Launch Enemy on taking damage
  (cast `/Game/Characters/Blueprint/BP_Alien` _returnvalue)
  (`self.LaunchCharacter` (* (`KismetMathLibrary.GetForwardVector` (`self.K2_GetActorRotation` _returnvalue)) 250.0))
  (set `TextBlock.Text` (`KismetTextLibrary.Conv_DoubleToText` Damage "HalfToEven") _damagetaken)
  (bind _isplayerdead_ (`/Game/Characters/Blueprint/Actor_Components/AC_PlayerStats.DecreasePlayerHealth` (`self.AC_PlayerStats`) Damage))
  (bind _output_get (set `self.Is Player Dead?` _isplayerdead_))
  (if _output_get
    (`self.BossDeath`)
    (`self.OnDeath`)
    (else
      (`KismetSystemLibrary.Delay` 1.0)
      (set `TextBlock.Text` "" _damagetaken))))

(event `TraceHit`
  ;[1 1 1] Sword Trace
  (bind (_outhit _returnvalue) (`KismetSystemLibrary.SphereTraceSingle` :`Start` (`SceneComponent.K2_GetComponentLocation` (`self.MaceTop`)) :`End` (`SceneComponent.K2_GetComponentLocation` (`self.MaceBottom`)) :`Radius` 6.5 :`TraceChannel` "TraceTypeQuery1" :`DrawTime` 1.0))
  (if _returnvalue
    (bind (_bblockinghit _binitialoverlap _time _distance _location _impactpoint _normal _impactnormal _physmat _hitactor) (`GameplayStatics.BreakHitResult` _outhit))
    (if (`self.ActorHasTag` _hitactor "Player")
      (`/Engine/EditorBlueprintResources/StandardMacros.DoOnce` false :!label _label
        (:`Completed`
          (`GameplayStatics.ApplyDamage` _hitactor (`self.Base Damage`) null null "/Script/Engine.DamageType")
          (bind _returnvalue_2 (`GameplayStatics.SpawnEmitterAtLocation` "/Game/VFX/Particles/Sparks/P_Sparks_C.P_Sparks_C" _location (`KismetMathLibrary.MakeRotFromXY` _normal _normal) (0.5 0.5 0.5) true "AutoRelease"))
          (bind _output_get (set `self.SparkEmitter` _returnvalue_2))
          (`KismetSystemLibrary.Delay` 0.5)
          (`ActorComponent.Deactivate` _output_get)
          (goto _label :!via `Reset`))))))

(event `self.ReceiveTick`
  (params (DeltaSeconds :type "Float (single-precision)"))
  ;[0.05098 0.05098 0.05098] Health Bar Face Camera
  (`self.K2_SetActorRotation` (`KismetMathLibrary.RInterpTo` (`self.K2_GetActorRotation`) (`KismetMathLibrary.FindLookAtRotation` (`self.K2_GetActorLocation`) (`self.K2_GetActorLocation` (`self.Player`))) (`GameplayStatics.GetWorldDeltaSeconds`))))

(event `self.ReceiveBeginPlay`
  ;[0.05098 0.05098 0.05098] Get Health Bar UI
  (bind _returnvalue (`|CreateWidget` "/Game/UI/BossUI/Boss_HUD.Boss_HUD_C"))
  (bind _output_get (set `self.BossHUD` _returnvalue))
  (`UserWidget.AddToViewport` _output_get 0)
  (bind _asbp_alien (cast `/Game/Characters/Blueprint/BP_Alien` (`GameplayStatics.GetPlayerCharacter` 0)))
  (set `self.Player` _asbp_alien))

(event `Attacks`
  (bind _attackanims (`self.AttackAnims`))
  ;[1 1 1] AI COMBO ATTACKS
  (`/Engine/EditorBlueprintResources/StandardMacros.DoOnce` false :!label _label_2
    (:`Completed`
      (`KismetSystemLibrary.Delay` (`KismetMathLibrary.RandomFloatInRange` 0.5 1.0))
      (`|PlayMontage` (`self.Mesh`) (`|GetArrayItem` _attackanims (`KismetMathLibrary.RandomInteger` (`KismetArrayLibrary.Array_Length` _attackanims))) 0.85
        (:`OnCompleted`
          (goto _label_2 :!via `Reset`))
        (:`OnInterrupted`
          (`KismetSystemLibrary.Delay` 1.0)
          (goto _label_2 :!via `Reset`))))))

(fn `Attack`
  (returns (`Anim Duration` :type "Float (double-precision)"))
  (if (not (`self.Is Player Dead?`))
    (`self.Attacks`)
    (return 0.4)))

(fn `IsDead?`
  (returns (IsDead :type Boolean))
  (return (`self.Is Player Dead?`)))

(fn `UserConstructionScript`)