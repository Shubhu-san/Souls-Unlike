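; BP_Normie is a melee enemy character with a floating health bar that turns toward the camera.
; Damage plays a hit montage, knocks it along the player's facing and reduces health through the reused ACPlayerStats component.
; On death it hides the bar, launches harder, plays death montage and sound, then destroys itself after a delay.
; Attack plays a DoOnce-gated montage while alive, re-arming on completion or randomly delayed after interruption.
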(event `self.ReceiveAnyDamage`
  (params (Damage :type "Float (single-precision)") (DamageType :type "DamageType Object Reference") (InstigatedBy :type "Controller Object Reference") (DamageCauser :type "Actor Object Reference"))
  (bind _returnvalue (`GameplayStatics.GetPlayerCharacter` 0))
  ;[0.05098 0.05098 0.05098] Damage]
  (`self.PlayAnimMontage` "/Game/Characters/Animation/Actions/AM_Hit_ImpactEnemy.AM_Hit_ImpactEnemy")
  ;;[0.05098 0.05098 0.05098] Launch Enemy on taking damage
  (cast `/Game/Characters/Blueprint/BP_Alien` _returnvalue)
  (`self.LaunchCharacter` (* (`KismetMathLibrary.GetForwardVector` (`self.K2_GetActorRotation` _returnvalue)) 250.0))
  (bind _isplayerdead_ (`/Game/Characters/Blueprint/Actor_Components/AC_PlayerStats.DecreasePlayerHealth` (`self.AC_PlayerStats`) Damage))
  (bind _output_get (set `self.Is Player Dead?` _isplayerdead_))
  (if _output_get
    ;;[0.05098 0.05098 0.05098] Enemy After Death
    (set `Widget.Visibility` "Hidden" (`self.EnemyUI`))
    (`self.PlayAnimMontage` "/Game/Characters/Animation/Actions/AM_Death.AM_Death")
    (`self.LaunchCharacter` (* (`KismetMathLibrary.GetForwardVector` (`self.K2_GetActorRotation` (`GameplayStatics.GetPlayerCharacter` 0))) 700.0))
    (`GameplayStatics.PlaySoundAtLocation` "/Game/Characters/Audio/Hit_Death/MS_Killed.MS_Killed" (`self.K2_GetActorLocation`) (struct) 1.0 1.0 0.0 null null null null)
    (`KismetSystemLibrary.Delay` 2.0)
    (`self.K2_DestroyActor`)))

(event `self.ReceiveTick`
  (params (DeltaSeconds :type "Float (single-precision)"))
  (bind _hp_bar (`self.Hp_Bar`))
  ;[0.05098 0.05098 0.05098] Health Bar Face Camera
  (`SceneComponent.K2_SetWorldRotation` _hp_bar (`KismetMathLibrary.FindLookAtRotation` (`SceneComponent.K2_GetComponentLocation` _hp_bar) (`SceneComponent.K2_GetComponentLocation` (`PlayerCameraManager.TransformComponent` (`GameplayStatics.GetPlayerCameraManager` 0)))) false false))

(event `self.ReceiveBeginPlay`
  ;[0.05098 0.05098 0.05098] Get Health Bar UI
  (bind _aswb_enemy_ui (cast `/Game/Characters/UI/EnemyUI/WB_EnemyUI` (`WidgetComponent.GetWidget` (`self.Hp_Bar`))))
  (set `self.EnemyUI` _aswb_enemy_ui))

(event `/Game/AI/BP_AI_BehaviourTrees.Attack`
  ;[0.05098 0.05098 0.05098] Attack On Melee Range
  (if (not (`self.Is Player Dead?`))
    (`/Engine/EditorBlueprintResources/StandardMacros.DoOnce` false :!label _label
      (:`Completed`
        (`|PlayMontage` (`self.Mesh`) "/Game/Characters/Animation/Attacks/Light/AM_LightMontage.AM_LightMontage"
          (:`OnCompleted`
            (goto _label :!via `Reset`))
          (:`OnInterrupted`
            (`KismetSystemLibrary.Delay` (`KismetMathLibrary.RandomFloatInRange` 0.8 1.8))
            (goto _label :!via `Reset`)))))))

(fn `UserConstructionScript`)